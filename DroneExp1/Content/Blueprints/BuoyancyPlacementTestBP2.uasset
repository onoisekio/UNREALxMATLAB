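; Test actor Blueprint that configures buoyancy on itself when constructed, with no active gameplay logic in the event graph.
; The Construction Script casts the root to a static mesh component, enables physics simulation, then adds a MyBuoyancyComponent to its owner.
; That component presets buoyancy, then takes the mesh to preset physics and add a pontoon.
; Debug prints report each stage, the pontoon result or a failed cast.
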(fn `UserConstructionScript`
  (bind _asstatic_mesh_component (cast `StaticMeshComponent` (`self.RootComponent`))
    (:`then`
      (`PrimitiveComponent.SetSimulatePhysics` _asstatic_mesh_component true)
      (`KismetSystemLibrary.PrintString` "Simulate Physics Check" true true (struct :`G` 1.0 :`B` 0.307804 :`A` 1.0) 5.0)
      (bind _returnvalue (`AddComponent|NODE_AddMyBuoyancyComponent-3` :`self` (`ActorComponent.GetOwner` _asstatic_mesh_component)))
      (`MyBuoyancyComponent.PresetBuoyancy` _returnvalue null)
      (`KismetSystemLibrary.PrintString` "Preset Buoyancy Done" true true (struct :`G` 1.0 :`B` 0.180421 :`A` 1.0) 5.0)
      (`MyBuoyancyComponent.PresetPhysics` _returnvalue _asstatic_mesh_component)
      (`KismetSystemLibrary.PrintString` "Preset Physics Done" true true (struct :`R` 0.064553 :`G` 1.0 :`A` 1.0) 5.0)
      (bind _returnvalue_2 (`MyBuoyancyComponent.AddPontoon` _returnvalue _asstatic_mesh_component))
      (`KismetSystemLibrary.PrintString` (`KismetStringLibrary.Conv_IntToString` _returnvalue_2) true true (struct :`G` 0.66 :`B` 1.0 :`A` 1.0) 5.0))
    (:`CastFailed`
      (`KismetSystemLibrary.PrintString` "StaticMeshComponent CAST FAILED" true true (struct :`R` 1.0 :`G` 0.01854 :`A` 1.0) 5.0))))